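; RoboHood's game instance, which wraps online session handling for hosting, joining and destroying multiplayer games.
; Hosting creates a LAN or online session sized by MaxPlayers, then after a short delay opens the chosen level as a listen server.
; Joining takes a session search result and prints debug or error messages.
; The network error handler is an empty stub, and the server list refresh call is unconnected.
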(event `Join Game Session`
  (params (GameSession :type "BlueprintSessionResult Structure"))
  ;[0.855 0.1026 0.1026] Join Session From Server List
  (`JoinSessionCallbackProxy.JoinSession` (`GameplayStatics.GetPlayerController` 0) GameSession
    (:`then`
      (`KismetSystemLibrary.PrintString` "Debug: Join Game Session Called"))
    (:`OnFailure`
      (`KismetSystemLibrary.PrintString` "Error: Session No Longer Exists" true true (struct :`R` 0.485 :`G` 0.072202 :`B` 0.062939 :`A` 1.0) 10.0))))

(event `HostGameSession`
  (params (LevelName :type Name) (IsLan :type Boolean))
  ;[0.855 0.1026 0.1026] Host Game Session
  (`CreateSessionCallbackProxy.CreateSession` (`GameplayStatics.GetPlayerController` 0) (`self.MaxPlayers`) IsLan
    (:`OnSuccess`
      (`KismetSystemLibrary.Delay` 2.0) ; Delay Loading Screen
      (`GameplayStatics.OpenLevel` LevelName true "listen"))))

(event `self.HandleNetworkError`
  (params (FailureType :type "ENetworkFailure Enum" :default "NetDriverAlreadyExists") (bIsServer :type Boolean))
  ;[0.855 0.1026 0.1026] Network Error
  (if bIsServer
    _))

(event `DestroyGameSession`
  ;[0.855 0.1026 0.1026] Destroy Game Session
  (`DestroySessionCallbackProxy.DestroySession` (`GameplayStatics.GetPlayerController` 0)))